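; AI controller for patrolling NPCs that runs BT_NPC and feeds it patrol and perception data through the Blackboard.
; BeginPlay copies loop and wait settings from the pawn's PatrolPath and sets the initial direction.
; Perception updates handle stimuli by array index: the first flags player sighting, the next two set investigation and target location, and none clears flags.
; It also holds health-based damage logic with an empty Death function.
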(event OnPerceptionUpdated(AIPerception)
  (params (UpdatedActors :type Array%20of%20Actor%20Object%20References))
  (for _array_element UpdatedActors
    (bind _info (Class|AIPerceptionComponent|GetActorsPerception (Variables|Default|GetAIPerception) _array_element))
    (CallFunction|HandleSenses (.lastsensedstimuli _info))))

(event EventBeginPlay
  (AI|RunBehaviorTree "/Game/Blueprints/ArtificialIntelligence/NPC/BT_NPC.BT_NPC")
  (bind _asbp_npc (Utilities|Casting|CastToBP_NPC (Pawn|GetControlledPawn)))
  (bind _output_get (Variables|Default|SetControlledPawn _asbp_npc))
  (AI|Components|Blackboard|SetValueasBool (AI|GetBlackboard 0) (Utilities|Name|MakeLiteralName "bIsPathLooping") (Variables|/Game/Blueprints/ArtificialIntelligence/NPC/BP_PatrolPath.BP_PatrolPath_C|GetbIsLooping (Variables|/Game/Blueprints/ArtificialIntelligence/NPC/BP_NPC.BP_NPC_C|GetPatrolPath _output_get)))
  (Class|BlackboardComponent|SetValueasInt (AI|GetBlackboard 0) (Utilities|Name|MakeLiteralName "Direction") 1)
  (AI|Components|Blackboard|SetValueasFloat (AI|GetBlackboard 0) (Utilities|Name|MakeLiteralName "WaitTime") (Variables|/Game/Blueprints/ArtificialIntelligence/NPC/BP_PatrolPath.BP_PatrolPath_C|GetWaitTime (Variables|/Game/Blueprints/ArtificialIntelligence/NPC/BP_NPC.BP_NPC_C|GetPatrolPath (Variables|Default|GetControlledPawn)))))

(fn ConstructionScript)

(fn HandleSenses
  (params (Array :type Array%20of%20AI%20Stimulus%20Structures))
  (for (_array_element _array_index) Array
    (LocalVariables|SetLocalSense _array_element)
    (switch int _array_index
      (:0
        (if (.bsuccessfullysensed (LocalVariables|GetLocalSense))
          (AI|Components|Blackboard|SetValueasBool (AI|GetBlackboard 0) (Utilities|Name|MakeLiteralName "bCanSeePlayer") (.bsuccessfullysensed (LocalVariables|GetLocalSense)))))
      (:1
        (if (.bsuccessfullysensed (LocalVariables|GetLocalSense))
          (AI|Components|Blackboard|SetValueasBool (AI|GetBlackboard 0) (Utilities|Name|MakeLiteralName "bIsInvestigating") (.bsuccessfullysensed (LocalVariables|GetLocalSense)))
          (AI|Components|Blackboard|SetValueasVector (AI|GetBlackboard 0) (Utilities|Name|MakeLiteralName "TargetLocation") (.stimuluslocation (LocalVariables|GetLocalSense)))))
      (:2
        (if (.bsuccessfullysensed (LocalVariables|GetLocalSense))
          (AI|Components|Blackboard|SetValueasBool (AI|GetBlackboard 0) (Utilities|Name|MakeLiteralName "bIsInvestigating") (.bsuccessfullysensed (LocalVariables|GetLocalSense)))
          (AI|Components|Blackboard|SetValueasVector (AI|GetBlackboard 0) (Utilities|Name|MakeLiteralName "TargetLocation") (.stimuluslocation (LocalVariables|GetLocalSense))))))))

(fn TakeDamage
  (params (Damage :type Float%20%28single-precision%29))
  (bind _output_get (Variables|Default|SetCurrentHealth (- (Variables|Default|GetCurrentHealth) Damage)))
  (if (<= _output_get 0.0)
    (CallFunction|Death)
    (else
      (bind _output_get_2 (Variables|Default|SetCurrentHealth (Math|Float|Clamp(Float) (Variables|Default|GetCurrentHealth) 0.0 (Variables|Default|GetHealthTotal))))
      (Development|PrintString (Utilities|String|ToString(Float) _output_get_2)))))

(fn Death)