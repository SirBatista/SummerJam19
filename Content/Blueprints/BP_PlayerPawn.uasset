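; Player vampire character with camera-relative movement, a dash, a taunt and a three-hit melee combo.
; Dash launches horizontally along camera-relative input, with a timeline driving speed and FOV while meshes swap, before a delayed reset.
; Attack montage notifies sphere-trace from alternating hands, reporting damage and messaging BPI_CombatInterface targets, while a retriggerable delay resets the combo.
; Taunts, dash endings and hits report noise or damage events to AI perception.
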(event Input|ActionEvents|InputActionDash
  (params (Key :type Key%20Structure))
  (bind _returnvalue (Transformation|GetActorLocation))
  (bind _returnvalue_2 (Input|AxisValues|GetMoveRight))
  (bind _returnvalue_3 (Input|AxisValues|GetMoveForward))
  (bind _followcamera (Variables|MyCharacter|GetFollowCamera))
  (bind _returnvalue_4 (Transformation|GetWorldRotation _followcamera))
  (bind (_roll _pitch _yaw) (Math|Rotator|BreakRotator _returnvalue_4))
  (bind _returnvalue_5 (Math|Rotator|MakeRotator _roll _pitch _yaw))
  (bind _returnvalue_6 (Math|Vector|GetRightVector _returnvalue_5))
  (bind _returnvalue_7 (Math|Vector|GetForwardVector _returnvalue_5))
  (bind _returnvalue_8 (* _returnvalue_6 _returnvalue_2))
  (bind _returnvalue_9 (* _returnvalue_7 _returnvalue_3))
  (bind _returnvalue_10 (+ _returnvalue_9 _returnvalue_8))
  (:Pressed
    (if (Variables|Default|GetbIsNotDashing?)
      (Components|Activation|Activate (Variables|Default|GetParticleSystem) true)
      (Rendering|SetVisibility (Variables|Character|GetMesh) false false)
      (Rendering|SetVisibility (Variables|Default|GetSkeletalMesh) true false)
      (Audio|PlaySoundatLocation "/Game/Sound/VampireDashIn_SCue.VampireDashIn_SCue" (Transformation|GetActorLocation) "0, 0, 0" 1.0 1.0 0.0 0 0 0)
      (Variables|Default|SetbIsNotDashing? false)
      (Class|NavMovementComponent|StopActiveMovement (Variables|Character|GetCharacterMovement))
      (Variables|Default|SetDashDirection (select (Math|Vector|Equal(Vector) _returnvalue_10 "0, 0, 0" 0.0001) (Math|Vector|GetForwardVector _returnvalue_5) _returnvalue_10))
      (bind (_direction _camerafieldofview _velocity) (Timeline|Timeline_Dash PlayFromStart)
        (:Update
          (Camera|SetFieldOfView (Variables|MyCharacter|GetFollowCamera) _camerafieldofview)
          (Character|LaunchCharacter (Math|Vector|MakeVector (.x (* (Variables|Default|GetDashDirection) (* _velocity (Variables|Default|GetDashSpeed)))) (.y (* (Variables|Default|GetDashDirection) (* _velocity (Variables|Default|GetDashSpeed)))) 0.0) true false))
        (:Finished
          (Utilities|FlowControl|Delay (Variables|Default|GetDashRefreshRate))
          (Variables|Default|SetbIsNotDashing? true)
          (Components|Activation|SetActive (Variables|Default|GetParticleSystem) true true)
          (Rendering|SetVisibility (Variables|Character|GetMesh) true false)
          (Rendering|SetVisibility (Variables|Default|GetSkeletalMesh) false false)
          (Audio|PlaySoundatLocation "/Game/Sound/VampireDashOut_SCue.VampireDashOut_SCue" _returnvalue "0, 0, 0" 1.0 1.0 0.0 0 0 0)
          (Class|AISenseHearing|ReportNoiseEvent _returnvalue 1.0 self 0.0 "Noise"))))))

(event Input|ActionEvents|InputActionAttack
  (params (Key :type Key%20Structure))
  (bind _returnvalue (Transformation|GetActorRotation))
  (bind _returnvalue_2 (Math|Vector|GetForwardVector _returnvalue))
  (:Pressed
    (if (not (Variables|Default|GetbIsAttacking?))
      (Variables|Default|SetbIsAttacking? true)
      (Animation|Montage|PlayMontage (Variables|Character|GetMesh) (Utilities|Select :Index (Variables|Default|GetAttackIndex) :Option%200 "/Game/Animations/TheCount/theCount_Attack1_Montage.theCount_Attack1_Montage" :Option%201 "/Game/Animations/TheCount/theCount_Attack2_Montage.theCount_Attack2_Montage" :Option%202 "/Game/Animations/TheCount/theCount_Attack3_Montage.theCount_Attack3_Montage")
        (:then
          (if (<= (Variables|Default|GetAttackIndex) 1)
            (Variables|Default|SetAttackIndex (+ (Variables|Default|GetAttackIndex) 1))
            (Utilities|FlowControl|Delay 0.5)
            (else
              (Variables|Default|SetAttackIndex 0)
              (Utilities|FlowControl|Delay 0.1)))
          (Variables|Default|SetbIsAttacking? false)
          (Utilities|FlowControl|RetriggerableDelay 0.8)
          (Variables|Default|SetAttackIndex 0))
        (:OnNotifyBegin
          (bind _outhit (Collision|SphereTraceByChannel (+ (Transformation|GetSocketLocation (Variables|Character|GetMesh) (Utilities|Select :Index (Variables|Default|GetAttackIndex) :Option%200 "LeftHand" :Option%201 "RightHand" :Option%202 "LeftHand")) (* _returnvalue_2 1e+02)) (+ (Transformation|GetSocketLocation (Variables|Character|GetMesh) (Utilities|Select :Index (Variables|Default|GetAttackIndex) :Option%200 "LeftHand" :Option%201 "RightHand" :Option%202 "LeftHand")) (* _returnvalue_2 1.5e+02)) 6e+01 "TraceTypeQuery2" false 0 "None"))
          (Class|AISenseDamage|ReportDamageEvent (.hitactor _outhit) self 1.0 (.tracestart _outhit))
          (if (Utilities|DoesObjectImplementInterface (.hitactor _outhit) "/Game/Blueprints/BPI_CombatInterface.BPI_CombatInterface_C")
            (Class|BPICombatInterface|ReceiveDamage(Message) (.hitactor _outhit) (Utilities|Select :Index (Variables|Default|GetAttackIndex) :Option%200 5.0 :Option%201 4.0 :Option%202 1e+01))))))))

(event Input|ActionEvents|InputActionCallOut
  (params (Key :type Key%20Structure))
  (bind _returnvalue (Transformation|GetActorLocation))
  (:Pressed
    (if (Variables|Default|GetbCanTaunt?)
      (Variables|Default|SetbCanTaunt? false)
      (Audio|PlaySoundatLocation "/Game/Sound/VampireLaugh_S.VampireLaugh_S" _returnvalue "0, 0, 0" 1.0 1.0 0.0 0 0 0)
      (Class|AISenseHearing|ReportNoiseEvent _returnvalue 1.0 self 0.0 "Noise")
      (Utilities|FlowControl|Delay 1.5)
      (Variables|Default|SetbCanTaunt? true))))

(event Input|AxisEvents|InputAxisLookUp
  (params (AxisValue :type Float%20%28single-precision%29))
  (Pawn|Input|AddControllerPitchInput AxisValue))

(event Input|AxisEvents|InputAxisTurn
  (params (AxisValue :type Float%20%28single-precision%29))
  (Pawn|Input|AddControllerYawInput AxisValue))

(event Input|AxisEvents|InputAxisMoveForward
  (params (AxisValue :type Float%20%28single-precision%29))
  (Pawn|Input|AddMovementInput (Math|Vector|GetForwardVector (Math|Rotator|MakeRotator 0.0 0.0 (.Yaw (Math|Rotator|BreakRotator (Pawn|GetControlRotation :!class /Script/Engine.Pawn))))) AxisValue false))

(event Input|AxisEvents|InputAxisMoveRight
  (params (AxisValue :type Float%20%28single-precision%29))
  (Pawn|Input|AddMovementInput (Math|Vector|GetRightVector (Math|Rotator|MakeRotator 0.0 0.0 (.Yaw (Math|Rotator|BreakRotator (Pawn|GetControlRotation :!class /Script/Engine.Pawn))))) AxisValue false))

(fn ConstructionScript)